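; BP_HeliBG1 is a background level piece for HeliRunner that also serves as an obstacle.
; Its construction script picks one of three HeliRunner level meshes at random and sets EmissiveStrength to zero on a dynamic material instance.
; CallIsObstacle reports it as an obstacle that overrides invincibility, so the player cannot go out of bounds while invincible.
; BeginPlay and Tick only call the parent class.
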(event `self.ReceiveBeginPlay`
  (`parent.ReceiveBeginPlay`))

(event `self.ReceiveTick`
  (params (DeltaSeconds :type "Float (single-precision)"))
  (`parent.ReceiveTick` DeltaSeconds))

(fn `CallIsObstacle`
  (returns (IsObstacle :type Boolean) (OverrideInvincibility :type Boolean))
  ;[0 0 0] This type of level piece should act as an obstacle and override invincibility to avoid player going out of bounds during invincibility duration.
  (return true true))

(fn `UserConstructionScript`
  (`parent.UserConstructionScript`)
  (`StaticMeshComponent.SetStaticMesh` (`self.StaticMesh`) (select `int` (`KismetMathLibrary.RandomIntegerInRange` 0 2) :`0` "/Game/EndlessRunnerCreator/HeliRunner/Meshes/SM_LevelPieceHeliRunner01.SM_LevelPieceHeliRunner01" :`1` "/Game/EndlessRunnerCreator/HeliRunner/Meshes/SM_LevelPieceHeliRunner02.SM_LevelPieceHeliRunner02" :`2` "/Game/EndlessRunnerCreator/HeliRunner/Meshes/SM_LevelPieceHeliRunner03.SM_LevelPieceHeliRunner03" :!type "StaticMesh Object Reference"))
  (bind _returnvalue (`PrimitiveComponent.CreateDynamicMaterialInstance` (`self.StaticMesh`) 0 null "None"))
  (`MaterialInstanceDynamic.SetScalarParameterValue` _returnvalue "EmissiveStrength" 0.0))