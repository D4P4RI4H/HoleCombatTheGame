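; BP_BGClouds is a background cloud actor for the Flappy Runner game.
; Its Construction Script randomly picks one of three cloud meshes and a yaw of 0 or 180 degrees for visual variety.
; It then sets LevelBoundsCollider's relative location from the mesh's world location plus bounds extent, multiplied by the actor's forward vector.
; The Event Graph has no active logic.
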(fn `UserConstructionScript`
  (locals (CurrentSpawnPoint :type "SceneComponent Object Reference"))
  (bind _staticmesh (`StaticMeshComponent.StaticMesh` (`self.StaticMesh`)))
  (bind (_returnvalue_origin _returnvalue_boxextent) (`KismetMathLibrary.BreakBoxSphereBounds` (`StaticMesh.GetBounds` _staticmesh)))
  (`parent.UserConstructionScript`)
  ;[0 0 0] Randomisation purely for visual improvements for variation
  (`StaticMeshComponent.SetStaticMesh` (`self.StaticMesh`) (select `int` (`KismetMathLibrary.RandomIntegerInRange` 0 2) :`0` "/Game/EndlessRunnerCreator/CommonAssets/Meshes/SM_Cloud1.SM_Cloud1" :`1` "/Game/EndlessRunnerCreator/CommonAssets/Meshes/SM_Cloud2.SM_Cloud2" :`2` "/Game/EndlessRunnerCreator/CommonAssets/Meshes/SM_Cloud3.SM_Cloud3" :!type "StaticMesh Object Reference"))
  (`SceneComponent.K2_SetWorldRotation` (`self.StaticMesh`) (`KismetMathLibrary.MakeRotator` 0.0 0.0 (`KismetMathLibrary.SelectFloat` 0.0 180.0 (`KismetMathLibrary.RandomBool`))) false false)
  ;[0 0 0] Check if static mesh has an asset set, if true:
  ; get the bounds of the mesh, + the location offset by the forward direction and set the LevelBoundsCollider.
  (`/Engine/EditorBlueprintResources/StandardMacros.IsValid` _staticmesh
    (:`Is Valid`
      (`SceneComponent.K2_SetRelativeLocation` (`self.LevelBoundsCollider`) (* (+ (`SceneComponent.K2_GetComponentLocation` (`self.StaticMesh`)) _returnvalue_boxextent) (`self.GetActorForwardVector`)) false false))))