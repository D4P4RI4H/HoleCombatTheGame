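; Player character for the Flappy Runner game that flaps upward on each press and falls under physics.
; Physics simulation on the collider starts when the level starts.
; If movement is allowed, a press zeroes velocity before an upward impulse so jumps stay consistent, then plays the jump montage, flap sound and Niagara effect.
; Tick smoothly pitches the actor from its vertical velocity.
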(event `self.ReceiveBeginPlay`
  (`parent.ReceiveBeginPlay`))

(event `self.ReceiveTick`
  (params (DeltaSeconds :type "Float (single-precision)"))
  (bind (_returnvalue_x _returnvalue_y _returnvalue_z) (`KismetMathLibrary.BreakVector` (`self.GetVelocity`)))
  (bind (_returnvalue_roll _returnvalue_pitch) (`KismetMathLibrary.BreakRotator` (`self.K2_GetActorRotation`)))
  ;[0 0 0] Update rotation based on velocity.
  (`self.K2_SetActorRotation` (`KismetMathLibrary.MakeRotator` 0.0 (`KismetMathLibrary.Lerp` _returnvalue_pitch (* _returnvalue_z 0.05) 0.05)) true))

(event `InputTouch`
  (params (Location :type "Vector Structure") (FingerIndex :type "ETouchIndex Enum"))
  ;[0 0 0] Touch and Desktop input.
  (:`Pressed`
    (if (`self.CanMove`)
      ;;[0 0 0] Reset current Velocity so Double Jump doesn't increase height exponentially. This makes sure all jumps fee the same to the player and more in control
      (`PrimitiveComponent.SetPhysicsLinearVelocity` (`self.CharacterCollider`) (0.0 0.0 0.0) false "None")
      (`PrimitiveComponent.AddImpulse` (`self.CharacterCollider`) (`KismetMathLibrary.MakeVector` 0.0 0.0 (`self.BaseImpulse`)) "None" true)
      ;[0 0 0] Play jump animation montage
      (`|PlayMontage` (`self.SkeletalMesh`) "/Game/EndlessRunnerCreator/CommonAssets/Animations/Jump_Cappy_Montage.Jump_Cappy_Montage" 1.0 0.0 "Default"
        (:`then`
          ;[0 0 0] Play the "flap" sound effect
          (`GameplayStatics.PlaySoundAtLocation` "/Game/EndlessRunnerCreator/FlappyRunner/Audio/Flap_Cue_Audio.Flap_Cue_Audio" (`self.K2_GetActorLocation`) (struct) 1.0 1.0 0.0 null null null)
          (`NiagaraFunctionLibrary.SpawnSystemAtLocation` "/Game/EndlessRunnerCreator/FlappyRunner/Effects/NS_FlappyFlap.NS_FlappyFlap" (`self.K2_GetActorLocation`)))))))

(fn `LevelStarted`
  (`parent.LevelStarted`)
  (`PrimitiveComponent.SetSimulatePhysics` (`self.CharacterCollider`) true))

(fn `UserConstructionScript`
  (`parent.UserConstructionScript`))