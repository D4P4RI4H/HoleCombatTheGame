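; Debris obstacle for the Voxel Runner endless runner, a child Blueprint that randomizes its own placement.
; It overrides the parent's random rotation with a fully random rotator, including roll.
; Its random location override keeps X and scatters the actor across Y and Z within hard-coded rough bounds of the level walls.
; Tick, construction and enabling only call the parent.
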(event `self.ReceiveTick`
  (params (DeltaSeconds :type "Float (single-precision)"))
  (`parent.ReceiveTick` DeltaSeconds))

(fn `EnableObject`
  (`parent.EnableObject`))

(fn `SetActorRandomLocation`
  (bind _returnvalue_x (`KismetMathLibrary.BreakVector` (`self.K2_GetActorLocation`)))
  (`parent.SetActorRandomLocation`)
  (`self.K2_SetActorLocation` (`KismetMathLibrary.MakeVector` _returnvalue_x (`KismetMathLibrary.RandomFloatInRange` -500.0 500.0) (`KismetMathLibrary.RandomFloatInRange` -500.0 500.0))))

(fn `SetActorRandomRotation`
  (`parent.SetActorRandomRotation`)
  (`self.K2_SetActorRotation` (`KismetMathLibrary.RandomRotator` true)))

(fn `UserConstructionScript`
  (`parent.UserConstructionScript`))