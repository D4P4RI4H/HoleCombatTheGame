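; Trail spawner variant of the spawner base for the endless runner, which wanders sideways along Y while it spawns.
; A looping timer picks a random Y target within the boundary.
; Tick steps toward that target at a fixed per-frame speed, not scaled by delta time, and clamps to the boundary.
; The spawn check adds a sphere overlap test to the parent's conditions, blocking spawns where objects already occupy the spot.
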(event `self.ReceiveBeginPlay`
  (`parent.ReceiveBeginPlay`)
  (`KismetSystemLibrary.K2_SetTimer` null "SetNewTargetPosition" (`self.RepositionFrequency`) true))

(event `self.ReceiveTick`
  (params (DeltaSeconds :type "Float (single-precision)"))
  (bind _boundary (`self.Boundary`))
  (bind _y (.y (`self.K2_GetActorLocation`)))
  (`self.K2_SetActorLocation` (`KismetMathLibrary.MakeVector` (.x (`self.K2_GetActorLocation`)) (`KismetMathLibrary.FClamp` (+ (* (`KismetMathLibrary.SignOfFloat` (- (`self.TargetPosition`) _y)) (`self.Speed`)) _y) (* _boundary -1.0) _boundary) (.z (`self.K2_GetActorLocation`)))))

(event `SetNewTargetPosition`
  (bind _boundary (`self.Boundary`))
  (set `self.TargetPosition` (`KismetMathLibrary.RandomFloatInRange` (* _boundary -1.0) _boundary)))

(fn `GetCanSpawnNewObject`
  (returns (ReturnValue :type Boolean))
  (bind (_outactors _returnvalue) (`KismetSystemLibrary.SphereOverlapActors` (`self.K2_GetActorLocation`) 75.0 (`|MakeArray` "ObjectTypeQuery1" "ObjectTypeQuery2" "ObjectTypeQuery4" :!type "EObjectTypeQuery Enum")))
  (return (and (not _returnvalue) (`parent.GetCanSpawnNewObject`))))

(fn `UserConstructionScript`
  (`parent.UserConstructionScript`))