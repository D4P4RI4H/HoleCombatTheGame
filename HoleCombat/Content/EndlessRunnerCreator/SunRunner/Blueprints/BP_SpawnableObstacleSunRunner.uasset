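; Spawnable obstacle for SunRunner that varies its look and animates in each time it is enabled.
; EnableObject picks a tall obstacle mesh or, rarely, a boulder, then randomizes per-axis scale and yaw before calling the parent.
; A timeline grows the actor from zero to full scale to hide pop-in.
; Random size goes on the mesh component, so the actor-level animation scales from the pivot.
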(event `self.ReceiveBeginPlay`
  (`parent.ReceiveBeginPlay`))

(event `AnimateObstacleScale`
  ;[0 0 0] Animate the scale of the prop. Avoids clear popping of obstacles appearing in the distance and looks cool.
  (bind (_direction _newtrack_0) (`Timeline|SpawnScaleAnim` :!via `PlayFromStart`)
    (:`Update`
      (`self.SetActorScale3D` (`KismetMathLibrary.VLerp` (0.0 0.0 0.0) (1.0 1.0 1.0) _newtrack_0)))))

(fn `EnableObject`
  ;[0 0 0] Randomise the object mesh, scale and rotations.
  (`self.SetRandomStaticMesh`)
  (`self.SetRandomActorScale`)
  (`self.SetRandomActorRotation`)
  ;[0 0 0] Animate object in
  (`self.AnimateObstacleScale`)
  (`parent.EnableObject`))

(fn `SetRandomActorRotation`
  (`self.K2_SetActorRotation` (`KismetMathLibrary.MakeRotator` 0.0 0.0 (`KismetMathLibrary.RandomFloatInRange` 0.0 360.0))))

(fn `SetRandomActorScale`
  (bind _returnvalue (`KismetMathLibrary.RandomFloatInRange` (`self.MinSize`) (`self.MaxSize`)))
  ;[0 0 0] Apply random scale to the static mesh. Apply it to the Mesh not the Object so we can make use of scaling from the pivot point to scale up and out from bottom/middle rather than middle/middle.
  (`SceneComponent.SetWorldScale3D` (`self.StaticMesh`) (`KismetMathLibrary.MakeVector` _returnvalue _returnvalue _returnvalue)))

(fn `SetRandomStaticMesh`
  (locals (bUseSpecialObstacleMesh :type Boolean :default false))
  (set `local.bUseSpecialObstacleMesh` (> (`KismetMathLibrary.RandomIntegerInRange` 0 10) 9))
  ;[0 0 0] Set the static mesh to a random mesh.
  (`StaticMeshComponent.SetStaticMesh` (`self.StaticMesh`) (select `int` (select `bool` (`local.bUseSpecialObstacleMesh`) :`true` 1) :`0` "/Game/EndlessRunnerCreator/VoxelRunner/Meshes/SM_ObstacleTallSunRunner.SM_ObstacleTallSunRunner" :`1` "/Game/EndlessRunnerCreator/CommonAssets/Meshes/SM_ObstacleBoulder.SM_ObstacleBoulder" :!type "StaticMesh Object Reference")))

(fn `UserConstructionScript`
  (`parent.UserConstructionScript`))