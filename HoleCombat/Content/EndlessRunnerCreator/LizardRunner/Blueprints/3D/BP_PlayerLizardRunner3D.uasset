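; BP_PlayerLizardRunner3D is the 3D player Blueprint for the LizardRunner game in Endless Runner Creator.
; It is a child Blueprint that defers BeginPlay and construction entirely to its parent.
; It extends the parent's JumpEffect and LandEffect events, calling each parent version and then playing the matching Cappy jump or land montage on the skeletal mesh.
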(event `self.ReceiveBeginPlay`
  (`parent.ReceiveBeginPlay`))

(event `self.JumpEffect`
  (`parent.JumpEffect`)
  ;[0 0 0] Play jump animation montage
  (`|PlayMontage` (`self.SkeletalMesh`) "/Game/EndlessRunnerCreator/CommonAssets/Animations/Jump_Cappy_Montage.Jump_Cappy_Montage" 1.0 0.0 "Default"))

(event `self.LandEffect`
  (`parent.LandEffect`)
  ;[0 0 0] Play land animation montage
  (`|PlayMontage` (`self.SkeletalMesh`) "/Game/EndlessRunnerCreator/CommonAssets/Animations/Land_Cappy_Montage.Land_Cappy_Montage" 1.0 0.0 "Default"))

(fn `UserConstructionScript`
  (`parent.UserConstructionScript`))